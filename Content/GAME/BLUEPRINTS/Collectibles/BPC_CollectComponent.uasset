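; BPC_CollectComponent is a component that handles picking up collectibles and adding their value to the score.
; On BeginPlay it caches the BP_GameInstance, which holds the score.
; Collect adds the collectible's Value to that score and destroys the collectible's owning actor.
; Each call also creates a new BPW_MainHUD widget and adds it to the viewport, without reusing or removing an earlier one.
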(event `self.ReceiveBeginPlay`
  (bind _asbp_game_instance (cast `/Game/GAME/BLUEPRINTS/Player/BP_GameInstance` (`GameplayStatics.GetGameInstance`)))
  (set `self.GameInstance` _asbp_game_instance))

(fn `Collect`
  (params (Collectible :type "/Game/GAME/BLUEPRINTS/Collectibles/BPC_CollectibleComponent Object Reference"))
  (bind _gameinstance (`self.GameInstance`))
  ;[0 1 0.2582] Update le score à chaque fois qu'une pièce est collectée
  (set `/Game/GAME/BLUEPRINTS/Player/BP_GameInstance.Score` (+ (`/Game/GAME/BLUEPRINTS/Collectibles/BPC_CollectibleComponent.Value` Collectible) (`/Game/GAME/BLUEPRINTS/Player/BP_GameInstance.Score` _gameinstance)) _gameinstance)
  ;[0 1 0.2582] Détruire l'object une fois récupérée et l'afficher dans l'HUD
  (`Actor.K2_DestroyActor` (`self.GetOwner` Collectible))
  (bind _returnvalue (`|CreateWidget` "/Game/GAME/WIDGET/BPW_MainHUD.BPW_MainHUD_C"))
  (`UserWidget.AddToViewport` _returnvalue 0))