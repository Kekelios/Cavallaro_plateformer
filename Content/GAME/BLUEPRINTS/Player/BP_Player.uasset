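; BP_Player is the player Blueprint, handling collectible pickup and interaction with world objects.
; On actor overlap, CollectObject looks for a BPC_CollectibleComponent on the other actor and passes it to BPCCollectComponent to collect.
; IA_Interact line-traces a short distance forward from FollowCamera on the Visibility channel and sends InteractMessage to hit actors implementing BPI_Interact.
; The Sphere overlap event is an empty stub.
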(event `self.ReceiveActorBeginOverlap`
  (params (OtherActor :type "Actor Object Reference"))
  (`|ExecutionSequence`
    (:`then_0`
      (`self.CollectObject` OtherActor))))

(event `self.Sphere.OnComponentBeginOverlap`
  (params (OverlappedComponent :type "PrimitiveComponent Object Reference") (OtherActor :type "Actor Object Reference") (OtherComp :type "PrimitiveComponent Object Reference") (OtherBodyIndex :type Integer) (bFromSweep :type Boolean) (SweepResult :type "HitResult Structure (by ref)"))
  ;[1 1 1] Ce code est bien pour une auto-intéraction
)

(event `EnhancedInput|/Game/ThirdPerson/Input/Actions/IA_Interact`
  (params (ActionValue :type Boolean) (ElapsedSeconds :type "Float (double-precision)") (TriggeredSeconds :type "Float (double-precision)") (InputAction :type "InputAction Object Reference" :default "/Game/ThirdPerson/Input/Actions/IA_Interact.IA_Interact"))
  (bind _followcamera (`self.FollowCamera`))
  (bind _returnvalue (`SceneComponent.K2_GetComponentLocation` _followcamera))
  ;[1 1 1] Intéragir avec un bouton, on utlise la caméra et le world location de cette même caméra pour savoir ou on est. Si la caméra est à bonne distance, elle intéragi avec le mesh de la porte
  (:`Triggered`
    (bind _outhit (`KismetSystemLibrary.LineTraceSingle` _returnvalue (+ _returnvalue (* (`SceneComponent.GetForwardVector` _followcamera) 500.0)) "TraceTypeQuery1"))
    (bind (_bblockinghit _binitialoverlap _time _distance _location _impactpoint _normal _impactnormal _physmat _hitactor) (`GameplayStatics.BreakHitResult` _outhit))
    (if (`KismetSystemLibrary.DoesImplementInterface` _hitactor "/Game/GAME/BLUEPRINTS/InteractBP/BPI_Interact.BPI_Interact_C")
      (message `/Game/GAME/BLUEPRINTS/InteractBP/BPI_Interact.Interact` _hitactor))))

(fn `CollectObject`
  (params (Target :type "Actor Object Reference"))
  (bind _returnvalue (`self.GetComponentByClass` Target "/Game/GAME/BLUEPRINTS/Collectibles/BPC_CollectibleComponent.BPC_CollectibleComponent_C"))
  (`/Engine/EditorBlueprintResources/StandardMacros.IsValid` _returnvalue
    (:`Is Valid`
      (`/Game/GAME/BLUEPRINTS/Collectibles/BPC_CollectComponent.Collect` (`self.BPC_CollectComponent`) _returnvalue))))

(fn `UserConstructionScript`
  (`parent.UserConstructionScript`))