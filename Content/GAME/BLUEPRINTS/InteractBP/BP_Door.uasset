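; BP_Door is an interactable door that swings open, closes itself and briefly lights a spotlight.
; Interact, intended as the BPI_interact hook, plays a timeline that yaws the door, then reverses it after a retriggerable delay.
; The same interaction shows the spotlight for a few seconds.
; Sphere overlap with BP_Player adds a BPW_InteractE prompt, and leaving clears all widgets.
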(event `OpenLight`
  ;[1 1 1] Light mais pas opti
  (`SceneComponent.SetVisibility` (`self.SpotLight`) true false)
  (`KismetSystemLibrary.Delay` 5.0)
  (`SceneComponent.SetVisibility` (`self.SpotLight`) false false))

(event `OpenDoor`
  ;[1 1 1] Faire une animation de porte : Ouverture/Fermeture
  (bind (_direction _alpha) (`Timeline|TM_door` :!label _label)
    (:`Update`
      (`SceneComponent.K2_SetRelativeRotation` (`self.Door`) (`KismetMathLibrary.MakeRotator` 0.0 0.0 (`KismetMathLibrary.Lerp` 0.0 90.0 _alpha)) false false))
    (:`Finished`
      (`KismetSystemLibrary.RetriggerableDelay` 2.0)
      (`self.CloseDoor`))))

(event `CloseDoor`
  ;[1 1 1] Faire une animation de porte : Ouverture/Fermeture
  (goto _label :!via `Reverse`))

(event `/Game/GAME/BLUEPRINTS/InteractBP/BPI_Interact.Interact`
  ;[1 1 1] Evenement avec le BPI_interact
  (`self.OpenDoor`)
  (`self.OpenLight`))

(event `self.Sphere.OnComponentBeginOverlap`
  (params (OverlappedComponent :type "PrimitiveComponent Object Reference") (OtherActor :type "Actor Object Reference") (OtherComp :type "PrimitiveComponent Object Reference") (OtherBodyIndex :type Integer) (bFromSweep :type Boolean) (SweepResult :type "HitResult Structure (by ref)"))
  ;[1 1 1] Code pas opti du tout pour afficher le widget
  (cast `/Game/GAME/BLUEPRINTS/Player/BP_Player` OtherActor)
  (bind _returnvalue (`|CreateWidget` "/Game/GAME/WIDGET/BPW_InteractE.BPW_InteractE_C"))
  (`UserWidget.AddToViewport` _returnvalue 0))

(event `self.Sphere.OnComponentEndOverlap`
  (params (OverlappedComponent :type "PrimitiveComponent Object Reference") (OtherActor :type "Actor Object Reference") (OtherComp :type "PrimitiveComponent Object Reference") (OtherBodyIndex :type Integer))
  ;[1 1 1] Code pas opti du tout pour afficher le widget
  (cast `/Game/GAME/BLUEPRINTS/Player/BP_Player` OtherActor)
  (`WidgetLayoutLibrary.RemoveAllWidgets`))

(fn `UserConstructionScript`)